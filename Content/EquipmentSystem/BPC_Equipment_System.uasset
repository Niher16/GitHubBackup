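; Equipment component for the BP_Test character that handles weapon pickup and the equipment menu.
; Interact sphere-traces forward from the follow camera, stores a hit BP_Weapon's item data in WeaponSlots and destroys the actor.
; The menu input toggles a lazily created, reused WB_Equipment widget, switching cursor and input mode.
; While the menu is open, the attack system is blocked and character movement is disabled.
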(event `self.ReceiveBeginPlay`
  ;[1 1 1] Begin
  (bind _asbp_test (cast `/Game/ThirdPerson/Characters/PC/BP_Test` (`self.GetOwner`)))
  (set `self.Follow Camera` (`/Game/ThirdPerson/Characters/PC/BP_Test.Follow Camera` _asbp_test))
  (set `self.BPC Attack System` (`/Game/ThirdPerson/Characters/PC/BP_Test.BPC_AttackSystem` _asbp_test)))

(event `EnhancedInput|/Game/ThirdPerson/Input/Actions/IA_Interact`
  (params (ActionValue :type Boolean) (ElapsedSeconds :type "Float (double-precision)") (TriggeredSeconds :type "Float (double-precision)") (InputAction :type "InputAction Object Reference" :default "/Game/ThirdPerson/Input/Actions/IA_Interact.IA_Interact"))
  (bind _follow_camera (`self.Follow Camera`))
  (bind _returnvalue (`SceneComponent.K2_GetComponentLocation` _follow_camera))
  ;[1 1 1] Pickup Trace
  (:`Started`
    (bind (_outhit _returnvalue_2) (`KismetSystemLibrary.SphereTraceSingleForObjects` :`Start` _returnvalue :`End` (+ _returnvalue (* (`KismetMathLibrary.GetForwardVector` (`SceneComponent.K2_GetComponentRotation` _follow_camera)) 1000.0)) :`Radius` 100.0 :`ObjectTypes` (`|MakeArray` "ObjectTypeQuery2" :!type "EObjectTypeQuery Enum") :`DrawDebugType` "ForDuration"))
    (if _returnvalue_2
      (bind _asbp_weapon (cast `/Game/EquipmentSystem/BP_Weapon` (`.HitActor` (`GameplayStatics.BreakHitResult` _outhit))))
      (`self.AddWeapon` (`/Game/EquipmentSystem/BP_Weapon.itemData` _asbp_weapon))
      (`Actor.K2_DestroyActor` _asbp_weapon))))

(event `EnhancedInput|/Game/ThirdPerson/Input/Actions/IA_Menu`
  (params (ActionValue :type Boolean) (ElapsedSeconds :type "Float (double-precision)") (TriggeredSeconds :type "Float (double-precision)") (InputAction :type "InputAction Object Reference" :default "/Game/ThirdPerson/Input/Actions/IA_Menu.IA_Menu"))
  (bind _returnvalue (`GameplayStatics.GetPlayerController` 0))
  (bind _bpc_attack_system (`self.BPC Attack System`))
  ;[1 1 1] Menu
  (:`Started`
    (if (not (`self.isPanelOpend?`))
      (set `/Game/ThirdPerson/Blueprints/BPC_AttackSystem.canAttack?` false _bpc_attack_system)
      (set `self.isPanelOpend?` true)
      (bind _equipment_widget (`self.Equipment Widget`)
        (:`then`
          (`Widget.SetVisibility` _equipment_widget "Visible"))
        (:`else`
          (bind _returnvalue_2 (`|CreateWidget` "/Game/EquipmentSystem/WB_Equipment.WB_Equipment_C"))
          (bind _output_get (set `self.Equipment Widget` _returnvalue_2))
          (`UserWidget.AddToViewport` _output_get 0)))
      (set `PlayerController.bShowMouseCursor` true _returnvalue)
      (`WidgetBlueprintLibrary.SetInputMode_GameAndUIEx` _returnvalue (`self.Equipment Widget`))
      (bind _asbp_test (cast `/Game/ThirdPerson/Characters/PC/BP_Test` (`self.GetOwner`)))
      (`CharacterMovementComponent.SetMovementMode` (`Character.CharacterMovement` _asbp_test) "MOVE_None" 0)
      (else
        (set `/Game/ThirdPerson/Blueprints/BPC_AttackSystem.canAttack?` true _bpc_attack_system)
        (set `self.isPanelOpend?` false)
        (bind _equipment_widget_2 (`self.Equipment Widget`)
          (:`then`
            (`Widget.SetVisibility` _equipment_widget_2 "Hidden")
            (set `PlayerController.bShowMouseCursor` false _returnvalue)
            (`WidgetBlueprintLibrary.SetInputMode_GameOnly` _returnvalue)
            (bind _asbp_test_2 (cast `/Game/ThirdPerson/Characters/PC/BP_Test` (`self.GetOwner`)))
            (`CharacterMovementComponent.SetMovementMode` (`Character.CharacterMovement` _asbp_test_2) "MOVE_Walking" 0))
          (:`else`))))))

(fn `AddWeapon`
  (params (NewItem :type "/Game/EquipmentSystem/S_Slots Structure (by ref)"))
  (`KismetArrayLibrary.Array_Add` (`self.weaponSlots`) NewItem))